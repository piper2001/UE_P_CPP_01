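; Turret-like spawner actor that periodically fires magic projectiles at the player.
; A looping timer started on BeginPlay spawns BP_SMagicProjectile at the actor's location, using the Arrow component's world rotation.
; Tick keeps that Arrow aimed at the first player pawn via a look-at rotation, so each shot heads toward the player's position at spawn time.
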(event `self.ReceiveBeginPlay`
  (`KismetSystemLibrary.K2_SetTimerDelegate` (delegate `SpawnProjectiles`) 2.0 true))

(event `SpawnProjectiles`
  (`|SpawnActorFromClass` "/Game/UE_CPP/BP_SMagicProjectile.BP_SMagicProjectile_C" (`KismetMathLibrary.MakeTransform` (`self.K2_GetActorLocation`) (`SceneComponent.K2_GetComponentRotation` (`self.Arrow`))) "Undefined" "OverrideRootScale" null null))

(event `self.ReceiveTick`
  (params (DeltaSeconds :type "Float (single-precision)"))
  (`SceneComponent.K2_SetWorldRotation` (`self.Arrow`) (`KismetMathLibrary.FindLookAtRotation` (`self.K2_GetActorLocation`) (`self.K2_GetActorLocation` (`GameplayStatics.GetPlayerPawn` 0))) false false))

(fn `UserConstructionScript`)